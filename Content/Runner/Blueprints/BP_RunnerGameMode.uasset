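; Game mode for a runner that builds and recycles an endless track of BP_Floor tiles.
; On BeginPlay it spawns a set number of tiles, each placed at the attach point returned by the previous one.
; ExtendFloor appends a new tile, then destroys and removes the oldest once the tile list exceeds that count by more than one, keeping the track length bounded.
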(event EventBeginPlay
  (for _index (range 0 (- (Variables|Default|GetNumberOfTiles) 1))
    (CallFunction|AddFloor)))

(event EventTick
  (params (DeltaSeconds :type Float%20%28single-precision%29)))

(fn ConstructionScript)

(fn AddFloor
  (bind _returnvalue (Game|SpawnActorfromClass "/Game/Runner/Blueprints/BP_Floor.BP_Floor_C" (Variables|Default|GetFloor%20AttachPoint) "Undefined" "MultiplyWithRoot" 0 0))
  (bind _returnvalue_2 (Default|GetAttachPoint _returnvalue))
  (Variables|Default|SetFloor%20AttachPoint _returnvalue_2)
  (Utilities|Array|Add (Variables|Default|GetFloorTiles) _returnvalue))

(fn ExtendFloor
  (bind _floortiles (Variables|Default|GetFloorTiles))
  (bind _output (Utilities|Array|Get(acopy) _floortiles))
  ;[1 1 1] Extend Floor tiles
  (CallFunction|AddFloor)
  (if (> (Utilities|Array|Length (Variables|Default|GetFloorTiles)) (+ (Variables|Default|GetNumberOfTiles) 1))
    (Actor|DestroyActor _output)
    (Utilities|Array|RemoveItem _floortiles _output)))